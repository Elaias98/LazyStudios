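; BP_HeroeBase is a hero Blueprint, apparently a prototype, that handles a melee input.
; IA_Melee Started and Completed share one path, setting Melee from the input value and the MeleeActivo gate, then matching the Sphere's visibility to it.
; That path then closes the gate and reopens it after a short Delay, acting as a cooldown on both press and release.
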(event Input|EnhancedActionEvents|EnhancedInputActionIA_Melee
  (params (ActionValue :type Boolean) (ElapsedSeconds :type Float%20%28double-precision%29) (TriggeredSeconds :type Float%20%28double-precision%29) (InputAction :type Input%20Action%20Object%20Reference :default "/Game/Blueprint/CharactersACTUALIZADO/InputActions/IA_Melee.IA_Melee"))
  (:Started
    (Variables|Default|SetMelee (and ActionValue (Variables|Default|GetMeleeActivo?)) :!label _label)
    (Rendering|SetVisibility (Variables|Default|GetSphere) (Variables|Default|GetMelee) false)
    (Variables|Default|SetMeleeActivo? false)
    (Utilities|FlowControl|Delay 0.6)
    (Variables|Default|SetMeleeActivo? true))
  (:Completed
    (goto _label)))

(event EventBeginPlay
  (|CallParentFunction) ; This node is disabled and will not be called.\nDrag off pins to build functionality.
)

(event Collision|EventActorBeginOverlap
  (params (OtherActor :type Actor%20Object%20Reference)))

(event EventTick
  (params (DeltaSeconds :type Float%20%28single-precision%29)))

(fn ConstructionScript
  (|CallParentFunction))