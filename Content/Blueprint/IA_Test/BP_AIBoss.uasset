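; AI controller for the boss that drives its behavior and tracks the player's hero through AI perception.
; On possess it runs the BT_BossIA behavior tree.
; Perception updates for BP_Heroe actors write the hero to a blackboard key when sensed and clear it when lost.
; Each sighting or loss also prints a Spanish debug message on screen.
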(event OnTargetPerceptionUpdated(AIPerception)
  (params (Actor :type Actor%20Object%20Reference) (Stimulus :type AI%20Stimulus%20Structure))
  (bind _asbp_heroe (Utilities|Casting|CastToBP_Heroe Actor))
  (if (.bsuccessfullysensed Stimulus)
    (AI|Components|Blackboard|SetValueasObject (AI|GetBlackboard 0) (Variables|Default|GetKey%20Name) _asbp_heroe)
    (Development|PrintString "Enemigo Avistado" true true "(R=0.543750,G=0.002036,B=0.000000,A=1.000000)")
    (else
      (AI|Components|Blackboard|SetValueasObject (AI|GetBlackboard 0) (Variables|Default|GetKey%20Name) 0)
      (Development|PrintString "Enemigo Perdido" true true "(R=0.543750,G=0.002036,B=0.000000,A=1.000000)"))))

(event EventBeginPlay)

(event EventTick
  (params (DeltaSeconds :type Float%20%28single-precision%29)))

(event EventPossess
  (params (PossessedPawn :type Pawn%20Object%20Reference))
  (AI|RunBehaviorTree "/Game/Blueprint/IA_Test/BT_BossIA.BT_BossIA"))

(fn ConstructionScript)