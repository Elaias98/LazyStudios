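; Melee enemy actor that attacks the hero and destroys itself, printing a message, when its health runs out.
; Each tick it copies health from its health component and sets the widget bar to VidaEnemigo divided by current health.
; FuncionAtaque plays a PaperZD attack override, with Ataca blocking re-entry until it completes or is cancelled.
; A separate hit-check event damages any BP_Heroe overlapping the melee attack area.
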(event EventBeginPlay)

(event EventTick
  (params (DeltaSeconds :type Float%20%28single-precision%29))
  (Utilities|FlowControl|Sequence
    (:then_0
      (bind _output_get (Variables|Default|SetVidaActualEnemigo (Variables|/Game/Blueprint/Componentes/BPC_ComponenteSalud.BPC_ComponenteSalud_C|GetVidaActualComponente (Variables|Default|GetBPC_ComponenteSalud))))
      (if (<= _output_get 0.0)
        (Development|PrintString "Enemigo eliminado" true true "(R=1.000000,G=0.091118,B=0.000000,A=1.000000)")
        (Actor|DestroyActor)))
    (:then_1
      (bind _aswbp_barra_enemigo (Utilities|Casting|CastToWBP_BarraEnemigo (UserInterface|GetUserWidgetObject (Variables|Default|GetWidget))))
      (Progress|SetPercent (Variables|/Game/Blueprint/Barras/WBP_BarraEnemigo.WBP_BarraEnemigo_C|GetProgressBar_205 _aswbp_barra_enemigo) (/ (Variables|Default|GetVidaEnemigo) (Variables|Default|GetVidaActualEnemigo))))))

(event EventChequearAtaqueEnemigoMelee
  (CallFunction|ChequearAtaqueEnemyMelee))

(event EventFuncionAtaque
  (if (not (Variables|Default|GetAtaca?))
    (|PlayAnimationOverridewithCallbacks (Variables|/Script/PaperZD.PaperZDAnimationComponent|GetAnimInstance (Variables|Default|GetAnimationComponent)) "/Game/Blueprint/CharactersACTUALIZADO/BlueprintsActores/Animaciones/AnimSequences/AtaqueLazyStudiosMelee.AtaqueLazyStudiosMelee" "DefaultSlot" 1.0 0.0
      (:then
        (Variables|Default|SetAtaca? true))
      (:OnCompleted
        (Variables|Default|SetAtaca? false :!label _label))
      (:OnCancelled
        (goto _label)))))

(fn ConstructionScript
  (|CallParentFunction))

(fn ChequearAtaqueEnemyMelee
  (for _array_element (Collision|GetOverlappingActors (Variables|Default|GetAtaqueMeleeEnemy) "/Game/Blueprint/CharactersACTUALIZADO/BlueprintsActores/BP_Heroe.BP_Heroe_C" :!class /Script/Engine.PrimitiveComponent)
    (Game|Damage|ApplyDamage _array_element (Variables|Default|GetDañoEnemigo) 0 0)))