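; AI controller for the melee enemy that tracks the player hero through perception.
; On possess it runs the BT_EnemyIA behavior tree.
; Perception updates on a BP_Heroe write the hero to a blackboard key when sensed and clear it when lost, printing a debug message for each case.
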(event OnTargetPerceptionUpdated(AIPerception)
  (params (Actor :type Actor%20Object%20Reference) (Stimulus :type AI%20Stimulus%20Structure))
  (bind _asbp_heroe (Utilities|Casting|CastToBP_Heroe Actor))
  (if (.bsuccessfullysensed Stimulus)
    (AI|Components|Blackboard|SetValueasObject (AI|GetBlackboard 0) (Variables|Default|GetKey%20Name) _asbp_heroe)
    (Development|PrintString "Objetivo Avistado")
    (else
      (AI|Components|Blackboard|SetValueasObject (AI|GetBlackboard 0) (Variables|Default|GetKey%20Name) 0)
      (Development|PrintString "Objetivo Perdido"))))

(event EventBeginPlay)

(event EventTick
  (params (DeltaSeconds :type Float%20%28single-precision%29)))

(event EventPossess
  (params (PossessedPawn :type Pawn%20Object%20Reference))
  (AI|RunBehaviorTree "/Game/Blueprint/IA_Test/AI_Melee/BT_EnemyIA.BT_EnemyIA"))

(fn ConstructionScript)