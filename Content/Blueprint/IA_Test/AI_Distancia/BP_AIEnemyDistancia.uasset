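; AI controller for the ranged enemy BP_EnemigoDistancia that runs the BT_DistanciaIA behavior tree on possession.
; On possession it also writes two locations to the Blackboard, built from the pawn's position plus per-enemy X/Y offsets at the same height.
; AI Perception sets BP_Heroe as the Blackboard target when sensed and clears it when lost, printing a debug message for each.
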(event OnTargetPerceptionUpdated(AIPerception)
  (params (Actor :type Actor%20Object%20Reference) (Stimulus :type AI%20Stimulus%20Structure))
  (bind _asbp_heroe (Utilities|Casting|CastToBP_Heroe Actor))
  (if (.bsuccessfullysensed Stimulus)
    (AI|Components|Blackboard|SetValueasObject (AI|GetBlackboard 0) (Variables|Default|GetKey%20Name_1) _asbp_heroe)
    (Development|PrintString "Vi al Objetivo")
    (else
      (AI|Components|Blackboard|SetValueasObject (AI|GetBlackboard 0) (Variables|Default|GetKey%20Name_1) 0)
      (Development|PrintString "Perdi El Objetivo"))))

(event EventBeginPlay)

(event EventTick
  (params (DeltaSeconds :type Float%20%28single-precision%29)))

(event EventPossess
  (params (PossessedPawn :type Pawn%20Object%20Reference))
  (AI|RunBehaviorTree "/Game/Blueprint/IA_Test/AI_Distancia/BT_DistanciaIA.BT_DistanciaIA")
  (bind _asbp_enemigo_distancia (Utilities|Casting|CastToBP_EnemigoDistancia PossessedPawn))
  (bind _returnvalue (CallFunction|PrimerUbicacion _asbp_enemigo_distancia _asbp_enemigo_distancia PossessedPawn))
  (AI|Components|Blackboard|SetValueasVector (AI|GetBlackboard 0) (Variables|Default|GetKey%20Name) _returnvalue)
  (bind _returnvalue_2 (CallFunction|SegundaUbicacion _asbp_enemigo_distancia _asbp_enemigo_distancia PossessedPawn))
  (AI|Components|Blackboard|SetValueasVector (AI|GetBlackboard 0) (Variables|Default|GetKey%20Name_0) _returnvalue_2))

(fn ConstructionScript)

(fn PrimerUbicacion
  (params (self2 :type BP%20Enemigo%20Distancia%20Object%20Reference) (self3 :type BP%20Enemigo%20Distancia%20Object%20Reference) (self4 :type Actor%20Object%20Reference))
  (bind _returnvalue (Transformation|GetActorLocation self4))
  (return (Math|Vector|MakeVector (+ (Variables|/Game/Blueprint/CharactersACTUALIZADO/BlueprintsActores/BP_EnemigoDistancia.BP_EnemigoDistancia_C|GetaPosicion_1_X self2) (.x _returnvalue)) (+ (Variables|/Game/Blueprint/CharactersACTUALIZADO/BlueprintsActores/BP_EnemigoDistancia.BP_EnemigoDistancia_C|GetbPosicion_1_Y self3) (.y _returnvalue)) (.z _returnvalue))))

(fn SegundaUbicacion
  (params (self2 :type BP%20Enemigo%20Distancia%20Object%20Reference) (self3 :type BP%20Enemigo%20Distancia%20Object%20Reference) (self4 :type Actor%20Object%20Reference))
  (bind _returnvalue (Transformation|GetActorLocation self4))
  (return (Math|Vector|MakeVector (+ (Variables|/Game/Blueprint/CharactersACTUALIZADO/BlueprintsActores/BP_EnemigoDistancia.BP_EnemigoDistancia_C|GetaPosicion_2_X self2) (.x _returnvalue)) (+ (Variables|/Game/Blueprint/CharactersACTUALIZADO/BlueprintsActores/BP_EnemigoDistancia.BP_EnemigoDistancia_C|GetbPosicion_2_Y self3) (.y _returnvalue)) (.z _returnvalue))))