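; Ranged enemy that attacks the hero by firing BP_ProyectilEnemigo projectiles.
; FuncionAtaque plays a PaperZD attack animation override and spawns the projectile at the enemy's transform, passing it the hero's location and a speed.
; An attacking flag blocks re-entry until the animation completes or is cancelled.
; BeginPlay casts the hero reference and fires one attack immediately, bypassing that check.
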(event EventBeginPlay
  (|CallParentFunction)
  (bind _asbp_heroe (Utilities|Casting|CastToBP_Heroe (Variables|Default|GetAs%20BP%20Heroe)))
  (|PlayAnimationOverridewithCallbacks (Variables|/Script/PaperZD.PaperZDAnimationComponent|GetAnimInstance (Variables|Default|GetAnimationComponent)) "/Game/Blueprint/CharactersACTUALIZADO/BlueprintsActores/Animaciones/AnimSequences/AtaqueLazyStudiosDistancia.AtaqueLazyStudiosDistancia" "DefaultSlot" 1.0 0.0
    (:then
      (Variables|Default|SetDistanciaEstaAtacando? true)
      (Development|PrintString "disparo")
      (Game|SpawnActorfromClass "/Game/Blueprint/CharactersACTUALIZADO/BlueprintsActores/BP_ProyectilEnemigo.BP_ProyectilEnemigo_C" (Transformation|GetActorTransform) "Undefined" "MultiplyWithRoot" 0 (Transformation|GetActorLocation _asbp_heroe) (Variables|Default|GetVelocidadProyectilEnemigo) 0))
    (:OnCompleted
      (Variables|Default|SetDistanciaEstaAtacando? false :!label _label))
    (:OnCancelled
      (goto _label))))

(event Collision|EventActorBeginOverlap
  (params (OtherActor :type Actor%20Object%20Reference))
  (|CallParentFunction OtherActor) ; This node is disabled and will not be called.\nDrag off pins to build functionality.
)

(event EventTick
  (params (DeltaSeconds :type Float%20%28single-precision%29)))

(event EventFuncionAtaque
  (if (not (Variables|Default|GetDistanciaEstaAtacando?))
    (|PlayAnimationOverridewithCallbacks (Variables|/Script/PaperZD.PaperZDAnimationComponent|GetAnimInstance (Variables|Default|GetAnimationComponent)) "/Game/Blueprint/CharactersACTUALIZADO/BlueprintsActores/Animaciones/AnimSequences/AtaqueLazyStudiosDistancia.AtaqueLazyStudiosDistancia" "DefaultSlot" 1.0 0.0
      (:then
        (Variables|Default|SetDistanciaEstaAtacando? true)
        (Development|PrintString "disparo")
        (Game|SpawnActorfromClass "/Game/Blueprint/CharactersACTUALIZADO/BlueprintsActores/BP_ProyectilEnemigo.BP_ProyectilEnemigo_C" (Transformation|GetActorTransform) "Undefined" "MultiplyWithRoot" 0 (Transformation|GetActorLocation (stale EventBeginPlay _asbp_heroe)) (Variables|Default|GetVelocidadProyectilEnemigo) 0))
      (:OnCompleted
        (Variables|Default|SetDistanciaEstaAtacando? false :!label _label))
      (:OnCancelled
        (goto _label)))))

(fn ConstructionScript
  (|CallParentFunction))