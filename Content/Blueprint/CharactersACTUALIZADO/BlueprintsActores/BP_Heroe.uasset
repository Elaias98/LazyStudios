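; Player hero character for a top-down game, with Enhanced Input movement, melee and projectile attacks, health and key-locked doors.
; A melee animation override blocks movement until it ends, overlap checks on Ataque damage melee and ranged enemies, and shots use a delay cooldown.
; BPCComponenteSalud handles healing and reports health drops, teleporting the hero to Localizacion at zero.
; Holding a key destroys the door; older damage logic remains disconnected and Tick prints health.
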(event Custom|ActualizarVida
  (params (Vida%20Actual :type Float%20%28double-precision%29) (VidaMaxima :type Float%20%28double-precision%29))
  ;[1 1 1] Set Location
  (bind _output_get (Variables|Default|SetVidaActual Vida%20Actual))
  (if (<= _output_get 0.0)
    (Transformation|SetActorLocation (Variables|Default|GetLocalizacion) false false)))

(event Input|EnhancedActionEvents|EnhancedInputActionAI_Move
  (params (ActionValue :type Vector%202D%20Structure) (ElapsedSeconds :type Float%20%28double-precision%29) (TriggeredSeconds :type Float%20%28double-precision%29) (InputAction :type Input%20Action%20Object%20Reference :default "/Game/Blueprint/CharactersACTUALIZADO/InputActions/AI_Move.AI_Move"))
  (bind (_x _y) (Math|Vector2D|BreakVector2D ActionValue))
  ;[0 1 0.04278] El movimiento se detiene cuando el Personaje Ataca
  (if (not (Variables|Default|GetSeUsoAtaque?))
    ;[0 1 0.034] MOVIEMIENTO
    (Variables|Default|SetDireccion ActionValue)
    (Pawn|Input|AddMovementInput "1.000000,0.000000,0.000000" _x false)
    (Pawn|Input|AddMovementInput "0.000000,1.000000,0.000000" _y false)))

(event Input|EnhancedActionEvents|EnhancedInputActionIA_Melee
  (params (ActionValue :type Boolean) (ElapsedSeconds :type Float%20%28double-precision%29) (TriggeredSeconds :type Float%20%28double-precision%29) (InputAction :type Input%20Action%20Object%20Reference :default "/Game/Blueprint/CharactersACTUALIZADO/InputActions/IA_Melee.IA_Melee"))
  ;[0.1531 1 0.0648] Ataque Melee
  (if (not (Variables|Default|GetSeUsoAtaque?))
    (|PlayAnimationOverridewithCallbacks (Variables|/Script/PaperZD.PaperZDAnimationComponent|GetAnimInstance (Variables|Default|GetAnimationComponent)) "/Game/Blueprint/CharactersACTUALIZADO/BlueprintsActores/Animaciones/AnimSequences/AtaqueLazyStudioPJ.AtaqueLazyStudioPJ" "DefaultSlot" 1.0 0.0
      (:then
        (Variables|Default|SetSeUsoAtaque? true))
      (:OnCompleted
        (Variables|Default|SetSeUsoAtaque? false :!label _label))
      (:OnCancelled
        (goto _label)))))

(event Input|EnhancedActionEvents|EnhancedInputActionIA_Shoot
  (params (ActionValue :type Boolean) (ElapsedSeconds :type Float%20%28double-precision%29) (TriggeredSeconds :type Float%20%28double-precision%29) (InputAction :type Input%20Action%20Object%20Reference :default "/Game/Blueprint/CharactersACTUALIZADO/InputActions/IA_Shoot.IA_Shoot"))
  ;[1 1 1] Proyectil
  (:Started
    (if (and ActionValue (Variables|Default|GetDispara?))
      (Game|SpawnActorfromClass "/Game/Blueprint/CharactersACTUALIZADO/BlueprintsActores/BP_Proyectil.BP_Proyectil_C" (Transformation|GetActorTransform) "Undefined" "MultiplyWithRoot" 0 "1.000000,0.000000,0.000000" (Variables|Default|GetVelocidadProyectil) 0)
      (Variables|Default|SetDispara? false)
      (Utilities|FlowControl|Delay 2.0)
      (Variables|Default|SetDispara? true))))

(event EventBeginPlay
  (|CallParentFunction)
  (bind _asplayer_controller (Utilities|Casting|CastToPlayerController (Pawn|GetController)))
  (Input|AddMappingContext (PlayerController|LocalPlayerSubsystems|GetEnhancedInputLocalPlayerSubsystem _asplayer_controller) "/Game/Blueprint/CharactersACTUALIZADO/InputActions/IMC_TopDownCharacter.IMC_TopDownCharacter" 0 "(bIgnoreAllPressedKeysUntilRelease=True,bForceImmediately=False,bNotifyUserSettings=False)")
  (bind _returnvalue (Actor|GetActorOfClass "/Game/Blueprint/BP_Puerta.BP_Puerta_C"))
  (Variables|Default|SetPuertaReferencia _returnvalue)
  (EventDispatchers|BindEventtoSebajoLavida (Variables|Default|GetBPC_ComponenteSalud) (delegate Custom|ActualizarVida)))

(event Collision|EventActorBeginOverlap
  (params (OtherActor :type Actor%20Object%20Reference))
  (|CallParentFunction OtherActor) ; This node is disabled and will not be called.\nDrag off pins to build functionality.
)

(event EventChequearAtaqueDistancia
  ;[1 0 0] Sistema Ataque-------------------------------CORREGIR! DEBERIA SER UN DAÑO GENERAL AL BP_ENEMIGO
  (CallFunction|ChequeoDañoDistancia))

(event EventChequearAtaque
  ;[1 0 0] Sistema Ataque-------------------------------CORREGIR! DEBERIA SER UN DAÑO GENERAL AL BP_ENEMIGO
  (CallFunction|ChequeoDaño))

(event EventVidaHeroe
  (params (CuracionRecibido :type Float%20%28double-precision%29))
  ;[1 1 1] PRUEBA COMPONENTE
  (Default|CurarVida (Variables|Default|GetBPC_ComponenteSalud) CuracionRecibido))

(event EventFuncionPuerta
  ;[0.07411 1 0.06793] Sistema Llave
  (if (stale EventFuncionLlave _output_get)
    (Actor|DestroyActor (stale EventFuncionLlave Puerta))
    (Variables|Default|SetAgarre%20Llave false)
    (else
      (Development|PrintString "Se Necesita llave"))))

(event EventFuncionLlave
  (params (AgarreLlave :type Boolean) (Puerta :type BP%20Puerta%20Object%20Reference))
  ;[0.07411 1 0.06793] Sistema Llave
  (bind _output_get (Variables|Default|SetAgarre%20Llave AgarreLlave))
  (if _output_get
    (Actor|DestroyActor Puerta)
    (Variables|Default|SetAgarre%20Llave false)
    (else
      (Development|PrintString "Se Necesita llave"))))

(event EventRecibirDaño
  (params (DañoTotal :type Float%20%28double-precision%29))
  ;[1 1 1] SISTEMA DE VIDA
)

(event EventTick
  (params (DeltaSeconds :type Float%20%28single-precision%29))
  ;[1 1 1] PRUEBA COMPONENTE
  (bind _output_get (Variables|Default|SetVidaActual (Variables|/Game/Blueprint/Componentes/BPC_ComponenteSalud.BPC_ComponenteSalud_C|GetVidaActualComponente (Variables|Default|GetBPC_ComponenteSalud))))
  (Development|PrintString (Utilities|String|ToString(Float) _output_get) true true "(R=0.000000,G=0.660000,B=1.000000,A=1.000000)" 1.0 "0"))

(fn ConstructionScript
  (|CallParentFunction))

(fn Curacion
  (params (CuracionRecibido :type Float%20%28double-precision%29))
  (bind _output_get (Variables|Default|SetVidaActual (+ CuracionRecibido (Variables|Default|GetVidaActual))))
  (Development|PrintString (Utilities|String|ToString(Float) _output_get) true true "(R=1.000000,G=0.000000,B=0.002630,A=1.000000)")
  (if (< _output_get 1e+02)
    (Development|PrintString "Sigue Curando")))

(fn ChequeoDaño
  (for _array_element (Collision|GetOverlappingActors (Variables|Default|GetAtaque) "/Game/Blueprint/IA_Test/Actores/BP_EnemigoMelee1.BP_EnemigoMelee1_C" :!class /Script/Engine.PrimitiveComponent)
    (Game|Damage|ApplyDamage _array_element (Variables|Default|GetDañoVar) 0 0)))

(fn ChequeoDañoDistancia
  (for _array_element (Collision|GetOverlappingActors (Variables|Default|GetAtaque) "/Game/Blueprint/CharactersACTUALIZADO/BlueprintsActores/BP_EnemigoDistancia.BP_EnemigoDistancia_C" :!class /Script/Engine.PrimitiveComponent)
    (Game|Damage|ApplyDamage _array_element (Variables|Default|GetDañoVar) 0 0)
    (Development|PrintString (Utilities|GetDisplayName _array_element))))

(fn GetVidaActual
  (return 0.0))